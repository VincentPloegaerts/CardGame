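; Player Blueprint for a card-based game, holding the player's potions and building the starting deck.
; On BeginPlay it sets itself as the owner reference on each potion, then creates the deck and shuffles the DeckManager's draw pile.
; CreateDeck constructs fixed numbers of Hit, Shield and Bash cards and adds them to the DeckManager.
; AddPotion and UsePotion only add or remove entries in the potion array.
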(event `self.ReceiveBeginPlay`
  (for _array_element (`self.Potions`)
    (set `/Game/Potions/Potion.PlayerRef` self _array_element))
  (`self.CreateDeck`)
  (`KismetArrayLibrary.Array_Shuffle` (`/Game/Cards/DeckManager.DrawPile` (`self.DeckManager`))))

(fn `AddPotion`
  (params (NewPotion :type "/Game/Potions/Potion Object Reference"))
  (`KismetArrayLibrary.Array_Add` (`self.Potions`) NewPotion))

(fn `CreateDeck`
  (for _ (range 5)
    (bind _returnvalue (`|GenericCreateObject` "/Game/Cards/HitCard.HitCard_C"))
    (`/Game/Cards/DeckManager.Add Card to Deck` (`self.DeckManager`) _returnvalue))
  (for _ (range 4)
    (bind _returnvalue_2 (`|GenericCreateObject` "/Game/Cards/ShieldCard.ShieldCard_C"))
    (`/Game/Cards/DeckManager.Add Card to Deck` (`self.DeckManager`) _returnvalue_2))
  (for _ (range 2)
    (bind _returnvalue_3 (`|GenericCreateObject` "/Game/Cards/BashCard.BashCard_C"))
    (`/Game/Cards/DeckManager.Add Card to Deck` (`self.DeckManager`) _returnvalue_3)))

(fn `UsePotion`
  (params (NewParam :type "/Game/Potions/Potion Object Reference (by ref)"))
  (`KismetArrayLibrary.Array_RemoveItem` (`self.Potions`) NewParam))

(fn `UserConstructionScript`)